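; BP_Enemy is an enemy actor that displays its health through a widget component using W_HUD_Enemy.
; BeginPlay caches the HUD widget, and Tick polls HealthComponent to set the health bar's percent.
; Each Tick also sets the widget component's visibility from the EnemysHUDCheck flag on the player tank pawn's widget controller.
; The Blueprint contains only this HUD logic, with no enemy behavior.
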(event EventBeginPlay
  (bind _asw_hud_enemy (Utilities|Casting|CastToW_HUD_Enemy (UserInterface|GetWidget (Variables|Default|GetWidget))))
  (Variables|Default|SetBP_Health _asw_hud_enemy))

(event Collision|EventActorBeginOverlap
  (params (OtherActor :type Actor%20Object%20Reference)))

(event EventTick
  (params (DeltaSeconds :type Float%20%28single-precision%29))
  (bind _returnvalue (Class|HealthComponent|GetHealthState (Variables|Default|GetHealthComponent)))
  (Progress|SetPercent (Variables|/Game/Core/Widgets/W_HUD_Enemy.W_HUD_Enemy_C|GetHP_Bar (Variables|Default|GetBP_Health)) _returnvalue)
  (bind _asbp_tank_pawn (Utilities|Casting|CastToBP_TankPawn (Game|Player|GetPlayerPawn 0)))
  (Rendering|SetVisibility (Variables|Default|GetWidget) (Variables|/Game/Core/Widgets/W_Widget_Controller.W_Widget_Controller_C|GetEnemysHUD_Check (Variables|/Game/Core/BP_TankPawn.BP_TankPawn_C|GetW_WidgetController _asbp_tank_pawn)) false))

(fn ConstructionScript)